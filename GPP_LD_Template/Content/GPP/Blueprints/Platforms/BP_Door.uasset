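; BP_Door is a door that slides from a start point to an end point when its OpenDoor event is called.
; BeginPlay snaps component S to StartPoint0 and sets the timeline play rate from MoveSpeed.
; OpenDoor plays the timeline, whose Alpha interpolates the world location of S toward EndPoint0 without sweeping.
; The graph has no closing logic or overlap trigger.
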(event Custom|OpenDoor
  (bind _alpha (Timeline|Timeline Play)
    (:Update
      (Transformation|SetWorldLocation (Variables|Default|Gets) (Math|Vector|Lerp(Vector) (Transformation|GetWorldLocation (Variables|Default|GetStartPoint_0)) (Transformation|GetWorldLocation (Variables|Default|GetEndPoint_0)) _alpha) false false))))

(event EventBeginPlay
  (Transformation|SetWorldLocation (Variables|Default|Gets) (Transformation|GetWorldLocation (Variables|Default|GetStartPoint_0)) false true)
  (Components|Timeline|SetPlayRate (Variables|Default|GetTimeline) (Variables|Default|GetMove%20Speed)))

(event Collision|EventActorBeginOverlap
  (params (OtherActor :type Actor%20Object%20Reference)))

(event EventTick
  (params (DeltaSeconds :type Float%20%28single-precision%29)))

(fn ConstructionScript)