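; BP_Trigger is a trigger box that temporarily switches the player's view to another camera.
; When BP_PlayerCharacter overlaps the box while Triggered is true, the view blends to Camera and character movement is disabled.
; After a Timer-length delay, it starts blending back to the player and immediately restores walking.
; Triggered is cleared only after that delay, so the sequence does not replay on later overlaps.
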(event OnComponentBeginOverlap(Box)
  (params (OverlappedComponent :type Primitive%20Component%20Object%20Reference) (OtherActor :type Actor%20Object%20Reference) (OtherComp :type Primitive%20Component%20Object%20Reference) (OtherBodyIndex :type Integer) (bFromSweep :type Boolean) (SweepResult :type Hit%20Result%20Structure%20%28by%20ref%29))
  (if (Variables|Default|GetTriggered)
    (bind _asbp_player_character (Utilities|Casting|CastToBP_PlayerCharacter OtherActor))
    (Class|CameraComponent|GetCameraView (Variables|/Game/GPP/Blueprints/Essential/BP_PlayerCharacter.BP_PlayerCharacter_C|GetFollowCamera _asbp_player_character) 0.0)
    (Game|Player|SetViewTargetwithBlend (Game|GetPlayerController 0) (Variables|Default|Getcamera) 5.0 "VTBlend_EaseIn" 0.5 false)
    (Pawn|Components|CharacterMovement|DisableMovement (Variables|/Script/Engine.Character|GetCharacterMovement _asbp_player_character))
    (Utilities|FlowControl|Delay (Variables|Default|GetTimer))
    (Game|Player|SetViewTargetwithBlend (Game|GetPlayerController 0) _asbp_player_character 5.0 "VTBlend_EaseOut" 0.8 false)
    (Pawn|Components|CharacterMovement|SetMovementMode (Variables|/Script/Engine.Character|GetCharacterMovement _asbp_player_character) "MOVE_Walking" 0)
    (Variables|Default|SetTriggered false)))

(event EventBeginPlay)

(event Collision|EventActorBeginOverlap
  (params (OtherActor :type Actor%20Object%20Reference)))

(event EventTick
  (params (DeltaSeconds :type Float%20%28single-precision%29)))

(fn ConstructionScript)