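; BP_BoomBot is a freezable NPC bot that patrols points, then chases its assigned target while a fuse burns down and explodes.
; A state machine (Patrol, Waiting, Chase, Frozen) drives AIMoveTo movement, with Tick counting down random patrol waits and the fuse.
; The freezable component's callback halts movement and removes fuse VFX; once triggered, the bot resumes chasing on thaw with a reset fuse.
; At zero, the explodable component detonates and the actor is destroyed.
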(event Custom|GoToNextPatrolPoint
  ;[0.4491 0.8591 1] Patrol Logic
  (AI|AIMoveTo self "0, 0, 0" (Variables|Patrolling|GetTargetPoint) 25.0 false
    (:OnSuccess
      (CallFunction|ChangeState "NewEnumerator3"))))

(event Custom|OnFrozen
  (params (IsFrozen :type Boolean))
  ;[0.4491 0.8591 1] Init
  ;;[0.4491 0.8591 1] Bind to freeze notification
  (if IsFrozen
    (CallFunction|ChangeState "NewEnumerator2")
    (else
      (CallFunction|ChangeState "NewEnumerator0"))))

(event Custom|SetTarget
  (params (Target :type BP%20Player%20Character%20Object%20Reference))
  ;[0.4491 0.8591 1] Set Target
  (bind _output_get (Variables|Explosion|SetTarget Target))
  (if (== _output_get 0)
    (AI|Navigation|StopMovement (Pawn|GetController))
    (else
      (CallFunction|ChangeState "NewEnumerator1"))))

(event Custom|StartExploding
  ;[0.4491 0.8591 1] Explode
  (Variables|Explosion|SetFuse%20Timer (Variables|Explosion|GetFuse%20Time))
  (if (== (Variables|Default|GetFuseParticle) 0)
    (bind _returnvalue (Niagara|SpawnSystemAttached "/Game/GPP/Particles/NS_Fuse.NS_Fuse" (Variables|Character|GetMesh) "Fuse" "0, 0, 0" "0.000000,-90.000000,90.000000" "SnapToTarget" false))
    (Variables|Default|SetFuseParticle _returnvalue)))

(event Custom|ChangeState
  (params (State :type E_BoomBotStates%20Enum :default "NewEnumerator0"))
  (bind _waittimeminmax (Variables|Patrolling|GetWaitTimeMinMax))
  ;[0.4491 0.8591 1] Change States
  (bind _output_get (Variables|Default|SetState State))
  (switch Utilities|FlowControl|Switch|SwitchonE_BoomBotStates _output_get
    (:NewEnumerator0
      (if (Variables|Explosion|GetHasStartedExploding)
        (CallFunction|ChangeState "NewEnumerator1")
        (else
          (CallFunction|GotoNextPatrolPoint))))
    (:NewEnumerator1
      (CallFunction|StartExploding)
      (CallFunction|ChasePlayer)
      (Variables|Explosion|SetHasStartedExploding true))
    (:NewEnumerator2
      (AI|Navigation|StopMovement (Pawn|GetController))
      (bind _fuseparticle (Variables|Default|GetFuseParticle)
        (:then
          (Components|DestroyComponent _fuseparticle)
          (Variables|Default|SetFuseParticle 0))
        (:else)))
    (:NewEnumerator3
      (if (Variables|Explosion|GetHasStartedExploding)
        (CallFunction|ChangeState "NewEnumerator1")
        (else
          (Variables|Patrolling|SetWaitTimer (Math|Random|RandomFloatinRange (.x _waittimeminmax) (.y _waittimeminmax))))))))

(event Custom|ChasePlayer
  ;[0.4491 0.8591 1] Chase Logic
  (AI|AIMoveTo self "0, 0, 0" (Variables|Explosion|GetTarget) 25.0 false))

(event Custom|FinishedWaiting
  ;[0.4491 0.8591 1] Patrol Logic
  (CallFunction|SetNewTargetPoint)
  (CallFunction|ChangeState "NewEnumerator0"))

(event EventBeginPlay
  ;[0.4491 0.8591 1] Init
  (CallFunction|InitFreezableComp)
  ;;[0.4491 0.8591 1] Init Patrol
  (Variables|Patrolling|SetTargetPoint (Utilities|Array|Get(acopy) (Variables|Patrolling|GetPatrolPoints)))
  ;;[0.4491 0.8591 1] Bind to freeze notification
  (EventDispatchers|BindEventtoOnFrozenChanged (Variables|Default|GetBP_FreezableComponent) (delegate Custom|OnFrozen))
  (CallFunction|ChangeState "NewEnumerator0"))

(event EventDestroyed
  ;[0.4491 0.8591 1] Init
  ;;[0.4491 0.8591 1] Bind to freeze notification
  (EventDispatchers|UnbindEventfromOnFrozenChanged (Variables|Default|GetBP_FreezableComponent) (delegate Custom|OnFrozen)))

(event EventTick
  (params (DeltaSeconds :type Float%20%28single-precision%29))
  ;[0.4491 0.8591 1] Tick
  (switch Utilities|FlowControl|Switch|SwitchonE_BoomBotStates (Variables|Default|GetState)
    (:NewEnumerator1
      (CallFunction|DecreaseFuseTimer DeltaSeconds))
    (:NewEnumerator3
      (CallFunction|DecreaseWaitTimer DeltaSeconds))))

(fn ConstructionScript)

(fn InitFreezableComp
  (bind _mesh (Variables|Character|GetMesh))
  (bind _bp_freezablecomponent (Variables|Default|GetBP_FreezableComponent))
  (bind _returnvalue (Rendering|Material|CreateDynamicMaterialInstance (Rendering|Material|GetMaterial _mesh 0) "None" "None" :!class /Script/Engine.KismetMaterialLibrary))
  (Rendering|Material|SetMaterial _mesh 0 _returnvalue)
  (Default|InitMaterial _bp_freezablecomponent (Utilities|Array|MakeArray _returnvalue))
  (Default|InitFreezeStatus _bp_freezablecomponent))

(fn DecreaseFuseTimer
  (params (DeltaTime :type Float%20%28double-precision%29))
  (bind _output_get (Variables|Explosion|SetFuse%20Timer (- (Variables|Explosion|GetFuse%20Timer) DeltaTime)))
  (if (< _output_get 0.0)
    (Default|Explode (Variables|Default|GetBP_ExplodableComponent))
    (Actor|DestroyActor)))

(fn SetNewTargetPoint
  (bind _result (Math|Integer|IncrementInt (Variables|Patrolling|GetIndex))
    (:%20%20
      (bind _output_get (Variables|Patrolling|SetIndex _result))
      (if (>= _output_get (Utilities|Array|Length (Variables|Patrolling|GetPatrolPoints)))
        (Variables|Patrolling|SetIndex 0))
      (Variables|Patrolling|SetTargetPoint (Utilities|Array|Get(acopy) (Variables|Patrolling|GetPatrolPoints) (Variables|Patrolling|GetIndex))))))

(fn DecreaseWaitTimer
  (params (DeltaTime :type Float%20%28double-precision%29))
  (bind _output_get (Variables|Patrolling|SetWaitTimer (- (Variables|Patrolling|GetWaitTimer) DeltaTime)))
  (if (< _output_get 0.0)
    (CallFunction|FinishedWaiting)))